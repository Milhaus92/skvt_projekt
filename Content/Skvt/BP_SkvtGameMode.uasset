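; BP_SkvtGameMode is a game mode that handles respawning for the local player.
; On BeginPlay it caches player 0's controller as a BP_SkvtPlayerController.
; Respawn acts only when that controller has no valid pawn, possessing the character returned by FindCharacterToPossess or opening the menu if none is valid.
; FindCharacterToPossess simply delegates the choice of character to the player controller.
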(event `self.ReceiveBeginPlay`
  (bind _asbp_skvt_player_controller (cast `/Game/Skvt/Characters/BP_SkvtPlayerController` (`GameplayStatics.GetPlayerController` 0)))
  (set `self.PlayerController` _asbp_skvt_player_controller))

(event `Respawn`
  (bind _newcharacter (`self.FindCharacterToPossess`))
  (bind _playercontroller (`self.PlayerController`))
  (`/Engine/EditorBlueprintResources/StandardMacros.IsValid` (`Controller.K2_GetPawn` (`self.PlayerController`))
    (:`Is Not Valid`
      (`/Engine/EditorBlueprintResources/StandardMacros.IsValid` _newcharacter
        (:`Is Valid`
          (`Controller.Possess` _playercontroller _newcharacter))
        (:`Is Not Valid`
          (`/Game/Skvt/Characters/BP_SkvtPlayerController.Open Menu` _playercontroller))))))

(fn `FindCharacterToPossess`
  (returns (NewCharacter :type "Pawn Object Reference"))
  (return (`/Game/Skvt/Characters/BP_SkvtPlayerController.Get Character To Possess` :`self` (`self.PlayerController`))))

(fn `UserConstructionScript`)