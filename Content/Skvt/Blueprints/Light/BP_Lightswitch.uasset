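; BP_Lightswitch is an interactable light switch that toggles the point light of a referenced LightHolder.
; Entering its sphere enables player input and shows a tutorial widget for two seconds; leaving disables input and removes it.
; Pressing E plays audio and, if Switch is true, toggles the light and clears Switch, so it works only once.
; The branch that resets Switch and shows a "let there be light" tutorial is unconnected.
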(event `self.Sphere.OnComponentBeginOverlap`
  (params (OverlappedComponent :type "PrimitiveComponent Object Reference") (OtherActor :type "Actor Object Reference") (OtherComp :type "PrimitiveComponent Object Reference") (OtherBodyIndex :type Integer) (bFromSweep :type Boolean) (SweepResult :type "HitResult Structure (by ref)"))
  (`self.EnableInput` (`GameplayStatics.GetPlayerController` 0))
  (bind _returnvalue (`|CreateWidget` "/Game/Skvt/UI/Widgets/Tutorial/WBP_ToggleLightsTutorial.WBP_ToggleLightsTutorial_C"))
  (bind _output_get (set `self.ToggleLightsTutorialWidget` (`|MakeArray` _returnvalue)))
  (`UserWidget.AddToViewport` _output_get 0)
  (`KismetSystemLibrary.Delay` 2.0)
  (`Widget.RemoveFromParent` (`self.ToggleLightsTutorialWidget`)))

(event `self.Sphere.OnComponentEndOverlap`
  (params (OverlappedComponent :type "PrimitiveComponent Object Reference") (OtherActor :type "Actor Object Reference") (OtherComp :type "PrimitiveComponent Object Reference") (OtherBodyIndex :type Integer))
  (`self.DisableInput` (`GameplayStatics.GetPlayerController` 0))
  (`Widget.RemoveFromParent` (`self.ToggleLightsTutorialWidget`)))

(event `Key|E`
  (params (Key :type "Key Structure"))
  (:`Pressed`
    (`AddComponent|NODE_AddAudioComponent-0`)
    (if (`self.Switch`)
      (`SceneComponent.ToggleVisibility` (`PointLight.PointLightComponent` (`self.LightHolder`)) false)
      (set `self.Switch` false))))

(fn `UserConstructionScript`)