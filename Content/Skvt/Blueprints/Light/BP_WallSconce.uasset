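; BP_WallSconce is a wall sconce light with configurable brightness, color, spot cone angles and lit state.
; The construction script applies those settings to the SconceLight component and sets its visibility from IsLit.
; TurnOff hides the light unless IsDestroyed is set, via ToggleLightVisibility, which also stores IsLit.
; BeginPlay overwrites the Color variable with red but does not reapply it to the light.
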(event `self.ReceiveBeginPlay`
  (set `self.Color` (make `LinearColor` 1.0)))

(event `/Game/Skvt/Blueprints/BPI_Electric.Turn Off`
  (if (not (`self.IsDestroyed`))
    (`self.ToggleLightVisibility` false)))

(fn `InitLight`
  (bind _sconcelight (`self.SconceLight`))
  (`LightComponent.SetIntensity` _sconcelight (`self.Brightness`))
  (`LightComponent.SetLightColor` _sconcelight (`self.Color`) true)
  (`SpotLightComponent.SetInnerConeAngle` _sconcelight (`self.Inner Cone Angle`))
  (`SpotLightComponent.SetOuterConeAngle` _sconcelight (`self.Outer Cone Angle`)))

(fn `ToggleLightVisibility`
  (params (IsLit :type Boolean))
  (bind _output_get (set `self.IsLit` IsLit))
  (`SceneComponent.SetVisibility` (`self.SconceLight`) _output_get false))

(fn `UserConstructionScript`
  (`self.InitLight`)
  (`self.ToggleLightVisibility` (`self.IsLit`)))